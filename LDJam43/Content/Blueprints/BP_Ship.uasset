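; BP_Ship is the clickable ship actor for turn-based battles, serving as player ship, enemy or Zomborg variant.
; PositionID picks the class mesh and database upgrades for player and Zomborg ships, while other enemies roll stats from the current sector.
; Player clicks select, jump away or attack, and EnemyTakeTurn targets the taunter or a random player.
; Timed BP_Shot projectiles precede damage, specials, shield/mirror handling and destruction checks that update PC_LD43's turn and battle state.
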(event `HandleUpgrades`
  (bind _playercontroller (`self.PlayerController`))
  (bind _zomborg (`self.Zomborg`))
  (bind _health (`self.Health`))
  (bind _playercontroller_2 (`self.PlayerController`))
  (bind (_shipdatabase_assault _shipdatabase_tank _shipdatabase_tsunami _shipdatabase_medic _shipdatabase_castle) (break `/Game/Game/ShipDatabase` (`self.ShipDatabase`)))
  (bind (_upgrade_1 _upgrade_2 _upgrade_3) (break `/Game/Game/ShipUpgrades` (`|GetArrayItem` (`|MakeArray` _shipdatabase_assault _shipdatabase_tank _shipdatabase_tsunami _shipdatabase_medic _shipdatabase_castle) (`self.PositionID`))))
  (bind (_output_ships_min _output_ships_max _output_health_min _output_health_max _output_damage_min _output_damage_max) (break `/Game/Game/Sector` (`|GetArrayItem` (`.Sectors_4_CE031EA248878DFDF2D569909E71F132` (break `/Game/Game/SectorDatabase` (`self.SectorDatabase`))) (`/Game/Blueprints/BP_Location.Sector` (`/Game/Game/PC_LD43.Location_Current` _playercontroller_2)))))
  (if (`self.Enemy`)
    (if (`self.Zomborg`)
      (for (_array_element _array_index) (`|MakeArray` _upgrade_1 _upgrade_2 _upgrade_3) :!label _label
        (if (`|GetArrayItem` (`/Game/Game/PC_LD43.Upgrades` (`self.PlayerController`)) (+ (* (`self.PositionID`) 3) _array_index))
          (switch `/Game/Game/ENM_Upgrade` _array_element
            (:`NewEnumerator0`
              (set `self.TurnsPerRound` 2))
            (:`NewEnumerator1`
              (`/Engine/EditorBlueprintResources/StandardMacros.IncrementInt` (`self.Damage`)))
            (:`NewEnumerator3`
              (set `self.Health` (* _health 2)))
            (:`NewEnumerator5`
              (set `self.Health` (+ _health 2)))
            (:`NewEnumerator9`
              (if (not _zomborg)
                (set `/Game/Game/PC_LD43.ShieldActive` true _playercontroller)
                (set `/Game/Game/PC_LD43.ShieldAvailable` true _playercontroller)))
            (:`NewEnumerator10`
              (if (not _zomborg)
                (set `/Game/Game/PC_LD43.MirrorActive` true _playercontroller)
                (set `/Game/Game/PC_LD43.MirrorAvailable` true _playercontroller))))))
      (else
        (set `self.Health` (select `bool` (`/Game/Game/PC_LD43.Tutorial` _playercontroller_2) :`false` (`KismetMathLibrary.RandomIntegerInRange` _output_health_min _output_health_max) :`true` 3))
        (set `self.Damage` (`KismetMathLibrary.RandomIntegerInRange` _output_damage_min _output_damage_max))))
    (else
      (goto _label))))

(event `HandleSpecial`
  (params (Ship :type "/Game/Blueprints/BP_Ship Object Reference"))
  (bind _returnvalue (`self.K2_GetActorLocation`))
  (bind (_shipdatabase_assault _shipdatabase_tank _shipdatabase_tsunami _shipdatabase_medic _shipdatabase_castle) (break `/Game/Game/ShipDatabase` (`self.ShipDatabase`)))
  (bind _positionid (`/Game/Blueprints/BP_Ship.PositionID` Ship))
  (bind _enemyships (`self.EnemyShips`))
  (bind _enemyships_2 (`self.EnemyShips`))
  (bind _enemyships_3 (`self.EnemyShips`))
  (bind (_upgrade_1 _upgrade_2 _upgrade_3) (break `/Game/Game/ShipUpgrades` (`|GetArrayItem` (`|MakeArray` _shipdatabase_assault _shipdatabase_tank _shipdatabase_tsunami _shipdatabase_medic _shipdatabase_castle) _positionid)))
  (`|ExecutionSequence`
    (:`then_0`
      (goto _label_2 :!via `Reset`))
    (:`then_1`
      (for (_array_element _array_index) (`|MakeArray` _upgrade_1 _upgrade_2 _upgrade_3)
        (if (`|GetArrayItem` (`/Game/Game/PC_LD43.Upgrades` (`self.PlayerController`)) (+ (* _positionid 3) _array_index))
          (switch `/Game/Game/ENM_Upgrade` _array_element
            (:`NewEnumerator2`
              (set `self.Taunt` Ship))
            (:`NewEnumerator4`
              (`/Engine/EditorBlueprintResources/StandardMacros.DoOnce` false :!label _label_2
                (:`Completed`
                  (set `self.EnemiesLeft` 0)
                  (`KismetArrayLibrary.Array_Clear` _enemyships_3)
                  (for _array_element_2 (`/Game/Game/PC_LD43.OrderedShips` (`self.PlayerController`))
                    (if (`/Game/Blueprints/BP_Ship.Zomborg` Ship)
                      (bind _enemy (`/Game/Blueprints/BP_Ship.Enemy` _array_element_2))
                      (if (not _enemy)
                        (`/Engine/EditorBlueprintResources/StandardMacros.IncrementInt` (`self.EnemiesLeft`)
                          (:`  `
                            (`KismetArrayLibrary.Array_Add` _enemyships_3 _array_element_2))))
                      (elif _enemy
                        (`/Engine/EditorBlueprintResources/StandardMacros.IncrementInt` (`self.EnemiesLeft`)
                          (:`  `
                            (`KismetArrayLibrary.Array_Add` _enemyships_3 _array_element_2))))))
                  (if (== (`self.EnemiesLeft`) 1)
                    (set `self.Health` (- (`self.Health`) 2))
                    (`/Game/UI/W_HealthBar.SubtractHealth` (`self.HealthBar`) 2)
                    (else
                      (`KismetArrayLibrary.Array_RemoveItem` _enemyships_2 self)
                      (set `self.HighestDelay` 0.0)
                      (for _array_element_3 _enemyships_2
                        (bind _returnvalue_2 (`|SpawnActorFromClass` "/Game/Blueprints/BP_Shot.BP_Shot_C" (`KismetMathLibrary.MakeTransform` _returnvalue) "AlwaysSpawn" "OverrideRootScale" null _returnvalue (`self.K2_GetActorLocation` _array_element_3) false false 0.75 true null))
                        (bind _traveltime (`/Game/Blueprints/BP_Shot.CalculateTravelTime` _returnvalue_2))
                        (if (> _traveltime (`self.HighestDelay`))
                          (set `self.HighestDelay` _traveltime)))
                      (`KismetSystemLibrary.Delay` (`self.HighestDelay`))
                      (for _array_element_4 _enemyships_2
                        (`/Engine/EditorBlueprintResources/StandardMacros.DecrementInt` (`/Game/Blueprints/BP_Ship.Health` _array_element_4)
                          (:`  `
                            (`/Game/UI/W_HealthBar.SubtractHealth` (`/Game/Blueprints/BP_Ship.HealthBar` _array_element_4) 1)
                            (`self.CheckIfDestroyed` _array_element_4)))))))))
            (:`NewEnumerator6`
              (goto _label_2))
            (:`NewEnumerator7`
              (set `self.EnemiesLeft` 0)
              (`KismetArrayLibrary.Array_Clear` _enemyships)
              (for _array_element_5 (`/Game/Game/PC_LD43.OrderedShips` (`self.PlayerController`))
                (if (`/Game/Blueprints/BP_Ship.Zomborg` Ship)
                  (bind _enemy_2 (`/Game/Blueprints/BP_Ship.Enemy` _array_element_5))
                  (if (not (not _enemy_2))
                    (`/Engine/EditorBlueprintResources/StandardMacros.IncrementInt` (`self.EnemiesLeft`)
                      (:`  `
                        (`KismetArrayLibrary.Array_Add` _enemyships _array_element_5))))
                  (elif (not _enemy_2)
                    (`/Engine/EditorBlueprintResources/StandardMacros.IncrementInt` (`self.EnemiesLeft`)
                      (:`  `
                        (`KismetArrayLibrary.Array_Add` _enemyships _array_element_5))))))
              (for _array_element_6 _enemyships
                (bind _output_get (set `/Game/Blueprints/BP_Ship.Health` (`KismetMathLibrary.Clamp` (+ (`/Game/Blueprints/BP_Ship.Health` _array_element_6) 1) 0 (`/Game/Blueprints/BP_Ship.MaxHealth` _array_element_6)) _array_element_6))
                (`/Game/UI/W_HealthBar.AddHealth` (`/Game/Blueprints/BP_Ship.HealthBar` _array_element_6) _output_get)))
            (:`NewEnumerator8`
              (bind _output_get_2 (set `/Game/Blueprints/BP_Ship.Health` (`KismetMathLibrary.Clamp` (+ (`/Game/Blueprints/BP_Ship.Health` Ship) 1) 0 (`/Game/Blueprints/BP_Ship.MaxHealth` Ship)) Ship))
              (`/Game/UI/W_HealthBar.AddHealth` (`/Game/Blueprints/BP_Ship.HealthBar` Ship) _output_get_2))))))))

(event `self.ReceiveBeginPlay`
  (set `self.PlayerController` (cast `/Game/Game/PC_LD43` (`GameplayStatics.GetPlayerController` 0) :!pure true))
  (`self.HandleUpgrades`)
  (set `self.MaxHealth` (`self.Health`))
  (bind _returnvalue (`|CreateWidget` "/Game/UI/W_HealthBar.W_HealthBar_C" null (`self.Health`)))
  (`UserWidget.AddToViewport` _returnvalue 0)
  (`UserWidget.SetPositionInViewport` _returnvalue (`PlayerController.ProjectWorldLocationToScreen` (`self.PlayerController`) (+ (`self.K2_GetActorLocation`) (-2600.0 -2200.0 0.0)) false) true)
  (set `self.HealthBar` _returnvalue)
  (set `self.TurnsLeft` (`self.TurnsPerRound`))
  (set `self.StartPosition` (`self.K2_GetActorLocation`)))

(event `RemoveShields`
  (bind _positionid (`self.PositionID`))
  (bind _playercontroller (`self.PlayerController`))
  (if (== _positionid 4)
    (set `/Game/Game/PC_LD43.ShieldActive` false _playercontroller)
    (set `/Game/Game/PC_LD43.ShieldAvailable` false _playercontroller)
    (set `/Game/Game/PC_LD43.MirrorActive` false _playercontroller)
    (set `/Game/Game/PC_LD43.MirrorAvailable` false _playercontroller)
    (elif (== _positionid 1)
      (for _array_element (`/Game/Game/PC_LD43.OrderedShips` (`self.PlayerController`))
        (set `/Game/Blueprints/BP_Ship.Taunt` null _array_element)))))

(event `self.Box.OnBeginCursorOver`
  (params (TouchedComponent :type "PrimitiveComponent Object Reference")))

(event `BlockShipSelect`
  (params (Block :type Boolean))
  (for _array_element (`/Game/Game/PC_LD43.OrderedShips` (`self.PlayerController`))
    (set `/Game/Blueprints/BP_Ship.LockDeselect` Block _array_element)))

(event `CheckIfDestroyed`
  (bind _playercontroller (`self.PlayerController`))
  (if (<= (`self.Health`) 0)
    (`GameplayStatics.SpawnEmitterAtLocation` "/Game/StarterContent/Particles/P_Explosion.P_Explosion" (`self.K2_GetActorLocation`) (struct) (110.0 110.0 110.0))
    (`GameplayStatics.PlaySound2D` "/Game/Sound/Player_Destroy.Player_Destroy" 1.0 1.0 0.0 null null)
    (`self.SetActorHiddenInGame` true)
    (`KismetArrayLibrary.Array_RemoveItem` (`/Game/Game/PC_LD43.OrderedShips` _playercontroller) self)
    (`KismetSystemLibrary.Delay` 0.5)
    (if (`self.Enemy`)
      (`/Game/Game/PC_LD43.CheckIfEndBattle` _playercontroller false)
      (`Widget.RemoveFromParent` (`self.HealthBar`))
      (`self.K2_DestroyActor`)
      (else
        (`self.RemoveShields`)
        (`/Game/Game/PC_LD43.CheckIfEndBattle` _playercontroller true)
        (`KismetArrayLibrary.Array_Set` (`/Game/Game/PC_LD43.Ships_Health` _playercontroller) (`self.PositionID`))
        (if (> (`self.TurnsLeft`) 0)
          (`/Engine/EditorBlueprintResources/StandardMacros.DecrementInt` (`/Game/Game/PC_LD43.PlayerTurnsLeft` (`self.PlayerController`))
            (:`  `
              _)))
        (`Widget.RemoveFromParent` (`self.HealthBar`))
        (`self.CheckIfEndTurn`)
        (`self.K2_DestroyActor`)))))

(event `self.Box.OnEndCursorOver`
  (params (TouchedComponent :type "PrimitiveComponent Object Reference")))

(event `EnactTaunt`
  (bind _playercontroller (`self.PlayerController`))
  (bind _playercontroller_2 (`self.PlayerController`))
  (bind _currentship (`/Game/Game/PC_LD43.CurrentShip` (`self.PlayerController`)))
  (bind _playerturnsleft (`/Game/Game/PC_LD43.PlayerTurnsLeft` _playercontroller))
  (bind _returnvalue (`self.K2_GetActorLocation` (`/Game/Game/PC_LD43.CurrentShip` _playercontroller_2)))
  (bind _turnsleft (`/Game/Blueprints/BP_Ship.TurnsLeft` _currentship))
  (bind _damage (`/Game/Blueprints/BP_Ship.Damage` _currentship))
  (`self.BlockShipSelect` true :!label _label_3)
  (bind _returnvalue_2 (`|SpawnActorFromClass` "/Game/Blueprints/BP_Shot.BP_Shot_C" (`KismetMathLibrary.MakeTransform` _returnvalue) "Undefined" "OverrideRootScale" null _returnvalue (`self.K2_GetActorLocation`) false false 1.0 false null))
  (bind _traveltime (`/Game/Blueprints/BP_Shot.CalculateTravelTime` _returnvalue_2))
  (`KismetSystemLibrary.Delay` _traveltime)
  (`self.BlockShipSelect` false)
  (`/Game/Game/PC_LD43.RoundsTutorial` _playercontroller_2)
  (set `self.Health` (- (`self.Health`) _damage))
  (`/Game/UI/W_HealthBar.SubtractHealth` (`self.HealthBar`) _damage)
  (`self.HandleSpecial` _currentship)
  (`/Engine/EditorBlueprintResources/StandardMacros.DecrementInt` _turnsleft
    (:`  `
      (if (<= _turnsleft 0)
        (set `/Game/Blueprints/BP_Ship.TurnOver` true _currentship)
        (`SceneComponent.SetVisibility` (`/Game/Blueprints/BP_Ship.Selection` _currentship) false false)
        (`self.SelectShip` _currentship false)
        (set `/Game/Game/PC_LD43.CurrentShip` null _playercontroller)
        (`/Engine/EditorBlueprintResources/StandardMacros.DecrementInt` _playerturnsleft
          (:`  `
            (`KismetSystemLibrary.PrintString` (`KismetStringLibrary.Conv_IntToString` _playerturnsleft)))))
      (if (<= (`self.Health`) 0)
        (`self.CheckIfDestroyed`))
      (`self.CheckIfEndTurn`))))

(event `self.Box.OnClicked`
  (params (TouchedComponent :type "PrimitiveComponent Object Reference") (ButtonPressed :type "Key Structure"))
  (bind _playercontroller (`self.PlayerController`))
  (bind _playercontroller_2 (`self.PlayerController`))
  (bind _currentship (`/Game/Game/PC_LD43.CurrentShip` _playercontroller))
  (if (`/Game/Game/PC_LD43.Blocked` (`self.PlayerController`))
    _
    (elif (`self.LockDeselect`)
      _
      (elif (`self.Enemy`)
        (`/Engine/EditorBlueprintResources/StandardMacros.IsValid` (`/Game/Game/PC_LD43.CurrentShip` _playercontroller_2)
          (:`Is Valid`
            (goto _label_3)))
        (elif (`/Game/Game/PC_LD43.CanJump` _playercontroller_2)
          (`self.Jump`)
          (elif (not (`self.TurnOver`))
            (`/Engine/EditorBlueprintResources/StandardMacros.IsValid` _currentship
              (:`Is Valid`
                (`self.SelectShip` _currentship false))
              (:`Is Not Valid`
                _))
            (set `/Game/Game/PC_LD43.CurrentShip` self _playercontroller)
            (`self.SelectShip` true :!label _label_4)))))))

(event `CheckIfEndTurn`
  (bind _playercontroller (`self.PlayerController`))
  (if (<= (`/Game/Game/PC_LD43.PlayerTurnsLeft` _playercontroller) 0)
    (`/Game/Game/PC_LD43.EnemyTurn` _playercontroller)))

(event `FirstShip`
  (goto _label_4))

(event `EnemyTakeTurn`
  (bind _returnvalue (`self.K2_GetActorLocation`))
  (bind _playercontroller (`self.PlayerController`))
  (bind _playercontroller_2 (`self.PlayerController`))
  (bind _targettedplayer (`self.TargettedPlayer`))
  (bind _damage (`self.Damage`))
  (bind _taunt (`self.Taunt`))
  (bind _playercontroller_3 (`self.PlayerController`))
  (bind _playercontroller_4 (`self.PlayerController`))
  (bind _shieldavailable (`/Game/Game/PC_LD43.ShieldAvailable` _playercontroller))
  (bind _orderedships (`/Game/Game/PC_LD43.OrderedShips` _playercontroller_3))
  (bind _returnvalue_2 (`KismetMathLibrary.Clamp` (/ (`self.Damage`) 2) 1 999))
  (set `/Game/Game/PC_LD43.EnemyTakingTurn` true _playercontroller_3)
  (`/Engine/EditorBlueprintResources/StandardMacros.IsValid` _taunt
    (:`Is Valid`
      (set `self.TargettedPlayer` _taunt))
    (:`Is Not Valid`
      (bind _output_get (set `self.TargettedPlayer` (`|GetArrayItem` _orderedships (`KismetMathLibrary.RandomIntegerInRange` 0 (`KismetArrayLibrary.Array_LastIndex` _orderedships))) :!label _label_5))
      (if (`/Game/Blueprints/BP_Ship.Enemy` _output_get)
        (`KismetSystemLibrary.Delay` 0.0)
        (goto _label_5)
        (else
          _))))
  (`self.BlockShipSelect` true)
  (bind _returnvalue_3 (`|SpawnActorFromClass` "/Game/Blueprints/BP_Shot.BP_Shot_C" (`KismetMathLibrary.MakeTransform` _returnvalue) "AlwaysSpawn" "OverrideRootScale" null _returnvalue (`self.K2_GetActorLocation` _output_get) (`/Game/Game/PC_LD43.ShieldAvailable` _playercontroller_4) (`/Game/Game/PC_LD43.MirrorAvailable` _playercontroller_4) 1.0 false null))
  (bind _traveltime (`/Game/Blueprints/BP_Shot.CalculateTravelTime` _returnvalue_3))
  (`KismetSystemLibrary.Delay` _traveltime)
  (if (and (not _shieldavailable) (`self.Zomborg`))
    (`self.ZomborgSpecial` _output_get self))
  (`self.BlockShipSelect` false)
  (if _shieldavailable
    (set `/Game/Game/PC_LD43.ShieldAvailable` false _playercontroller)
    (`KismetSystemLibrary.PrintString` "Enemy fire shielded!")
    (if (`/Game/Game/PC_LD43.MirrorAvailable` _playercontroller_2)
      (set `/Game/Game/PC_LD43.MirrorAvailable` false _playercontroller_2)
      (`/Game/UI/W_HealthBar.SubtractHealth` (`self.HealthBar`) _returnvalue_2)
      (set `self.Health` (- (`self.Health`) _returnvalue_2))
      (`KismetSystemLibrary.PrintString` (`KismetStringLibrary.Concat_StrStr` "Enemy fire reflected for " (`KismetStringLibrary.Conv_IntToString` _returnvalue_2) " damage!"))
      (`self.CheckIfDestroyed`))
    (else
      (`/Game/UI/W_HealthBar.SubtractHealth` (`/Game/Blueprints/BP_Ship.HealthBar` _targettedplayer) _damage)
      (set `/Game/Blueprints/BP_Ship.Health` (- (`/Game/Blueprints/BP_Ship.Health` _targettedplayer) _damage) _targettedplayer)
      (`self.CheckIfDestroyed` _targettedplayer)
      (`KismetSystemLibrary.PrintString` "Enemy fired!")))
  (set `/Game/Game/PC_LD43.EnemyTakingTurn` false _playercontroller_2))

(event `Jump`
  (bind _playercontroller (`self.PlayerController`))
  (for _array_element (`/Game/Game/PC_LD43.OrderedShips` (`self.PlayerController`))
    (if (not (`/Game/Blueprints/BP_Ship.Enemy` _array_element))
      (`PrimitiveComponent.SetMaterial` (`/Game/Blueprints/BP_Ship.Selection` _array_element) 0 "/Game/Materials/M_TestEmit_Green.M_TestEmit_Green")))
  (set `/Game/Game/PC_LD43.CanJump` false _playercontroller)
  (`/Engine/EditorBlueprintResources/StandardMacros.DecrementInt` (`/Game/Game/PC_LD43.PlayerTurnsLeft` _playercontroller)
    (:`  `
      (`self.RemoveShields`)
      (`KismetArrayLibrary.Array_RemoveItem` (`/Game/Game/PC_LD43.OrderedShips` _playercontroller) self)
      (`/Game/Game/PC_LD43.CheckIfEndBattle` _playercontroller true)
      (`Widget.RemoveFromParent` (`self.HealthBar`))
      (`self.K2_DestroyActor`))))

(event `ZomborgSpecial`
  (params (Ship :type "/Game/Blueprints/BP_Ship Object Reference"))
  (`self.HandleSpecial` Ship))

(fn `SelectShip`
  (params (Selected :type Boolean))
  (`PrimitiveComponent.SetMaterial` (`self.Selection`) 0 (select `bool` Selected :`false` "/Game/Materials/M_TestEmit_Green.M_TestEmit_Green" :`true` "/Game/Materials/M_TestEmit_Blue.M_TestEmit_Blue" :!type "MaterialInterface Object Reference"))
  (return))

(fn `UserConstructionScript`
  (bind _positionid (`self.PositionID`))
  (if (`self.Enemy`)
    (`SceneComponent.SetVisibility` (`self.Selection`) false false)
    (`SceneComponent.SetVisibility` (`self.Stink`) true false)
    (if (`self.Zomborg`)
      (`StaticMeshComponent.SetStaticMesh` (`self.Cube`) (select `int` _positionid :`0` "/Game/Meshes/Assault.Assault" :`1` "/Game/Meshes/Tank.Tank" :`2` "/Game/Meshes/Tsunami.Tsunami" :`3` "/Game/Meshes/Medic.Medic" :`4` "/Game/Meshes/Castle.Castle" :!type "StaticMesh Object Reference") :!label _label)
      (`SceneComponent.SetVisibility` (`self.Cone`) false false)
      (`TimelineComponent.SetPlayRate` (`self.IdleAnim`) (select `int` _positionid :`0` 1.5 :`1` 0.25 :`2` 0.5 :`3` 1.0 :`4` 0.75 :!type "Float (single-precision)"))
      (else
        (`StaticMeshComponent.SetStaticMesh` (`self.Cube`) "/Game/Meshes/Zomborg.Zomborg")
        (`SceneComponent.SetVisibility` (`self.Cone`) false false)))
    (else
      (goto _label))))