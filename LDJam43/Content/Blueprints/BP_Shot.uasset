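; BP_Shot is a projectile actor that travels in a straight line from a start location to an end location, then destroys itself.
; On BeginPlay, it divides distance by Speed to get travel time and sets the Lerp timeline's play rate to the inverse.
; The timeline's alpha interpolates the actor's location without sweeping.
; A FadeIn timeline that would scale the sphere is never triggered.
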(event `self.ReceiveBeginPlay`
  (bind _traveltime (`self.CalculateTravelTime`))
  (`TimelineComponent.SetPlayRate` (`self.Lerp`) (/ 1.0 _traveltime))
  (bind (_direction _alpha) (`Timeline|Lerp` :!via `PlayFromStart`)
    (:`Update`
      (`self.K2_SetActorLocation` (`KismetMathLibrary.VLerp` (`self.StartLocation`) (`self.EndLocation`) _alpha)))
    (:`Finished`
      (`self.K2_DestroyActor`))))

(fn `CalculateTravelTime`
  (returns (TravelTime :type "Float (double-precision)"))
  (return (/ (`KismetMathLibrary.VSize` (- (`self.EndLocation`) (`self.StartLocation`))) (`self.Speed`))))

(fn `UserConstructionScript`)