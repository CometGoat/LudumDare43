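; BP_EnemyForce is the enemy force actor that advances and retreats along a line of map positions in an LD43 game.
; Each event blocks the player controller while a timeline lerps the actor along Y, retreating twice the advance distance and index count.
; When movement finishes, it unblocks input and starts a battle if the player's position index is at or below its own.
; The Advance and Retreat sound cues are swapped relative to event names.
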(event `self.ReceiveBeginPlay`
  (set `self.PlayerController` (cast `/Game/Game/PC_LD43` (`GameplayStatics.GetPlayerController` 0) :!pure true)))

(event `Advance`
  (bind _startlocation (`self.StartLocation`))
  (bind _currentpositionindex (`self.CurrentPositionIndex`))
  (bind _playercontroller (`self.PlayerController`))
  (set `/Game/Game/PC_LD43.Blocked` true (`self.PlayerController`))
  (set `self.StartLocation` (`self.K2_GetActorLocation`))
  (`GameplayStatics.PlaySound2D` "/Game/Sound/Zomborg_Retreat.Zomborg_Retreat" 1.0 1.0 0.0 null null)
  (bind (_direction _alpha) (`Timeline|Advancer` :!via `PlayFromStart`)
    (:`Update`
      (`self.K2_SetActorLocation` (`KismetMathLibrary.VLerp` _startlocation (+ _startlocation (0.0 500.0 0.0)) _alpha)))
    (:`Finished`
      (set `/Game/Game/PC_LD43.Blocked` false (`self.PlayerController`))
      (`/Engine/EditorBlueprintResources/StandardMacros.IncrementInt` _currentpositionindex
        (:`  `
          (if (<= (`/Game/Blueprints/BP_Location.PositionIndex` (`/Game/Game/PC_LD43.Location_Current` _playercontroller)) _currentpositionindex)
            (`/Game/Game/PC_LD43.StartBattle` _playercontroller true)))))))

(event `Retreat`
  (bind _currentpositionindex (`self.CurrentPositionIndex`))
  (bind _playercontroller (`self.PlayerController`))
  (bind _startlocation (`self.StartLocation`))
  (set `/Game/Game/PC_LD43.Blocked` true (`self.PlayerController`))
  (set `self.StartLocation` (`self.K2_GetActorLocation`))
  (`GameplayStatics.PlaySound2D` "/Game/Sound/Zomborg_Advance.Zomborg_Advance" 1.0 1.0 0.0 null null)
  (bind (_direction _alpha) (`Timeline|Timeline_0` :!via `PlayFromStart`)
    (:`Update`
      (`self.K2_SetActorLocation` (`KismetMathLibrary.VLerp` _startlocation (+ _startlocation (0.0 -1000.0 0.0)) _alpha)))
    (:`Finished`
      (set `/Game/Game/PC_LD43.Blocked` false (`self.PlayerController`))
      (`/Engine/EditorBlueprintResources/StandardMacros.DecrementInt` _currentpositionindex
        (:`  `
          (`/Engine/EditorBlueprintResources/StandardMacros.DecrementInt` _currentpositionindex
            (:`  `
              (if (<= (`/Game/Blueprints/BP_Location.PositionIndex` (`/Game/Game/PC_LD43.Location_Current` _playercontroller)) _currentpositionindex)
                (`/Game/Game/PC_LD43.StartBattle` _playercontroller true)))))))))

(fn `UserConstructionScript`)