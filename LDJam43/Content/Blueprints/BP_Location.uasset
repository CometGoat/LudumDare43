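; BP_Location is a clickable map location that reports hover and click travel choices to the PC_LD43 player controller.
; On BeginPlay it registers itself as the current location if flagged as the start.
; Locations whose position index is in the upgrade positions roll a random core ID that sets the sphere's red, green or blue emissive material.
; Sphere cursor events update the controller's highlighted or current location, then call its suggest or travel function.
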(event `HandleUpgrade`
  (if (`KismetArrayLibrary.Array_Contains` (`self.UpgradePositions`) (`self.PositionIndex`))
    (bind _output_get (set `self.CoreID` (`KismetMathLibrary.RandomIntegerInRange` 0 2)))
    (`PrimitiveComponent.SetMaterial` (`self.Sphere`) 0 (select `int` _output_get :`0` "/Game/Materials/M_TestEmit_Red.M_TestEmit_Red" :`1` "/Game/Materials/M_TestEmit_Green.M_TestEmit_Green" :`2` "/Game/Materials/M_TestEmit_Blue.M_TestEmit_Blue" :!type "MaterialInterface Object Reference"))))

(event `self.ReceiveBeginPlay`
  (`self.HandleUpgrade`)
  (bind _output_get (set `self.PlayerController` (cast `/Game/Game/PC_LD43` (`GameplayStatics.GetPlayerController` 0) :!pure true)))
  (if (`self.StartLocation`)
    (set `/Game/Game/PC_LD43.Location_Current` self _output_get)))

(event `self.Sphere.OnBeginCursorOver`
  (params (TouchedComponent :type "PrimitiveComponent Object Reference"))
  (bind _playercontroller (`self.PlayerController`))
  (if (not (== (`/Game/Game/PC_LD43.Location_Highlighted` _playercontroller) self))
    (set `/Game/Game/PC_LD43.Location_Highlighted` self _playercontroller)
    (`/Game/Game/PC_LD43.SuggestNewLocation` _playercontroller)))

(event `self.Sphere.OnClicked`
  (params (TouchedComponent :type "PrimitiveComponent Object Reference") (ButtonPressed :type "Key Structure"))
  (bind _playercontroller (`self.PlayerController`))
  (if (not (== (`/Game/Game/PC_LD43.Location_Current` _playercontroller) self))
    (set `/Game/Game/PC_LD43.Location_Current` self _playercontroller)
    (`/Game/Game/PC_LD43.TravelToNewLocation` _playercontroller)))

(fn `UserConstructionScript`)