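; Camera Blueprint that also handles the game's exploration and battle music, plus a screen distortion effect.
; Both tracks start on BeginPlay and keep playing, while SwapMusic uses a timeline to crossfade their volumes by the Battle flag, leaving the inactive track faintly audible.
; Distort runs a second timeline that rewrites the camera's post-process settings, animating an intensity value alongside fixed vignette and grain.
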(event `self.ReceiveBeginPlay`
  (`AudioComponent.Play` (`self.Explore`) 0.0)
  (`AudioComponent.Play` (`self.Battle`) 0.0))

(event `SwapMusic`
  (params (Battle :type Boolean))
  (bind (_direction _alpha) (`Timeline|Music` :!via `PlayFromStart`)
    (:`Update`
      (bind _returnvalue (`KismetMathLibrary.Lerp` 0.05 1.0 _alpha))
      (bind _returnvalue_2 (`KismetMathLibrary.Lerp` 1.0 0.05 _alpha))
      (`AudioComponent.SetVolumeMultiplier` (`self.Explore`) (select `bool` Battle :`false` _returnvalue :`true` _returnvalue_2))
      (`AudioComponent.SetVolumeMultiplier` (`self.Battle`) (select `bool` Battle :`false` _returnvalue_2 :`true` _returnvalue)))))

(event `Distort`
  (bind (_direction _max) (`Timeline|DistortTime` :!via `PlayFromStart`)
    (:`Update`
      (set `CameraComponent.PostProcessSettings` (make `PostProcessSettings` :`SceneFringeIntensity` _max :`VignetteIntensity` 0.5 :`GrainJitter` 0.5 :`GrainIntensity` 0.5) (`self.Camera`)))))

(fn `UserConstructionScript`)